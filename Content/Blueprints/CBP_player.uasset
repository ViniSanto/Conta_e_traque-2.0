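; First-person player character with look, movement and rate-limited shooting, where refilling ammo means answering an equation quiz.
; Firing on empty reveals a display and three answer panels; the player cycles the highlighted slot and confirms.
; A correct answer refills ammo and generates a new puzzle, while a wrong one costs health.
; SlotRespostasErradas randomizes digit, neighboring wrong answers and slot, driving the visuals through Material Parameter Collections.
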(event Input|EnhancedActionEvents|EnhancedInputActionIA_move
  (params (ActionValue :type Vector%202D%20Structure) (ElapsedSeconds :type Float%20%28double-precision%29) (TriggeredSeconds :type Float%20%28double-precision%29) (InputAction :type Input%20Action%20Object%20Reference :default "/Game/Input/Action/IA_move.IA_move"))
  (:Triggered
    (Pawn|Input|AddMovementInput (Math|Vector|GetRightVector (Variables|Collision|GetCapsuleComponent)) (.x ActionValue) false)
    (Pawn|Input|AddMovementInput (Math|Vector|GetForwardVector (Variables|Collision|GetCapsuleComponent)) (.y ActionValue) false))
  (:Started
    (Variables|Default|SetAndando true))
  (:Completed
    (Variables|Default|SetAndando false)))

(event Input|EnhancedActionEvents|EnhancedInputActionIA_look
  (params (ActionValue :type Vector%202D%20Structure) (ElapsedSeconds :type Float%20%28double-precision%29) (TriggeredSeconds :type Float%20%28double-precision%29) (InputAction :type Input%20Action%20Object%20Reference :default "/Game/Input/Action/IA_look.IA_look"))
  (bind _returnvalue (* (.y ActionValue) -1.0))
  (Transformation|AddLocalRotation (Variables|Collision|GetCapsuleComponent) (Math|Rotator|MakeRotator 0.0 0.0 (.x ActionValue)) false false)
  (if (> _returnvalue 0.0)
    (if (< (.pitch (Transformation|GetWorldRotation (Variables|Default|GetCamera))) 85.0)
      (Transformation|AddLocalRotation (Variables|Default|GetCamera) (Math|Rotator|MakeRotator 0.0 _returnvalue 0.0) false false))
    (elif (> (.pitch (Transformation|GetWorldRotation (Variables|Default|GetCamera))) -85.0)
      (Transformation|AddLocalRotation (Variables|Default|GetCamera) (Math|Rotator|MakeRotator 0.0 _returnvalue 0.0) false false))))

(event Input|EnhancedActionEvents|EnhancedInputActionIA_tiro
  (params (ActionValue :type Boolean) (ElapsedSeconds :type Float%20%28double-precision%29) (TriggeredSeconds :type Float%20%28double-precision%29) (InputAction :type Input%20Action%20Object%20Reference :default "/Game/Input/Action/IA_tiro.IA_tiro"))
  (:Triggered
    (Variables|Default|SetTtiro (+ (Variables|Default|GetTtiro) (Variables|Default|GetDelta%20Seconds)))
    (if (> (Variables|Default|GetTtiro) (Variables|Default|GetPeriodoTiro))
      (Variables|Default|SetTtiro 0.0)
      (if (> (Variables|Default|GetMunicao) 0)
        (Variables|Default|SetMunicao (- (Variables|Default|GetMunicao) 1))
        (Development|PrintString "tiro")
        (Game|SpawnActorfromClass "/Game/Blueprints/ABP_tiro.ABP_tiro_C" (Math|Transform|MakeTransform (Transformation|GetSocketLocation (Variables|Default|GetBracosFP) "arma_ponta") (Transformation|GetWorldRotation (Variables|Default|GetCamera)) "1.000000,1.000000,1.000000") "AlwaysSpawn" "MultiplyWithRoot" 0 0)
        (Animation|Montage|MontagePlay (Components|SkeletalMesh|GetAnimInstance (Variables|Default|GetBracosFP)) "/Game/Personagens/AM_heroi_atirando.AM_heroi_atirando" 2.0 "MontageLength" 0.0 true)
        (else
          (Rendering|SetVisibility (Variables|Default|Getplaca2) true false)
          (if (== (Variables|Default|GetslotChoice) 0)
            (Rendering|SetVisibility (Variables|Default|Getcontorno0) true false)
            (elif (== (Variables|Default|GetslotChoice) 1)
              (Rendering|SetVisibility (Variables|Default|Getcontorno1) true false)
              (elif (== (Variables|Default|GetslotChoice) 2)
                (Rendering|SetVisibility (Variables|Default|Getcontorno2) true false))))))))
  (:Started
    (Variables|Default|SetShooting true))
  (:Completed
    (Variables|Default|SetShooting false)))

(event Input|EnhancedActionEvents|EnhancedInputActionIA_select
  (params (ActionValue :type Float%20%28double-precision%29) (ElapsedSeconds :type Float%20%28double-precision%29) (TriggeredSeconds :type Float%20%28double-precision%29) (InputAction :type Input%20Action%20Object%20Reference :default "/Game/Input/Action/IA_select.IA_select"))
  (if (== (Variables|Default|GetMunicao) 0)
    (Variables|Default|SetslotChoice (Math|Integer|%(Integer) (+ (Variables|Default|GetslotChoice) (Math|Float|Truncate (Math|Float|Sign(Float) ActionValue)) 3) 3))
    (if (== (Variables|Default|GetslotChoice) 0)
      (Rendering|SetVisibility (Variables|Default|Getcontorno0) true false)
      (Rendering|SetVisibility (Variables|Default|Getcontorno1) false false)
      (Rendering|SetVisibility (Variables|Default|Getcontorno2) false false)
      (elif (== (Variables|Default|GetslotChoice) 1)
        (Rendering|SetVisibility (Variables|Default|Getcontorno0) false false)
        (Rendering|SetVisibility (Variables|Default|Getcontorno1) true false)
        (Rendering|SetVisibility (Variables|Default|Getcontorno2) false false)
        (elif (== (Variables|Default|GetslotChoice) 2)
          (Rendering|SetVisibility (Variables|Default|Getcontorno0) false false)
          (Rendering|SetVisibility (Variables|Default|Getcontorno1) false false)
          (Rendering|SetVisibility (Variables|Default|Getcontorno2) true false))))))

(event Input|EnhancedActionEvents|EnhancedInputActionIA_confirmar
  (params (ActionValue :type Boolean) (ElapsedSeconds :type Float%20%28double-precision%29) (TriggeredSeconds :type Float%20%28double-precision%29) (InputAction :type Input%20Action%20Object%20Reference :default "/Game/Input/Action/IA_confirmar.IA_confirmar"))
  (if (== (Variables|Default|Getslotchoice) (Variables|Default|GetSlot))
    (Development|PrintString "acertou")
    (Variables|Default|SetMunicao (Variables|Default|GetmaxMunicao))
    (Rendering|SetVisibility (Variables|Default|Getcontorno0) false false)
    (Rendering|SetVisibility (Variables|Default|Getcontorno1) false false)
    (Rendering|SetVisibility (Variables|Default|Getcontorno2) false false)
    (Rendering|SetVisibility (Variables|Default|Getplaca0) false false)
    (Rendering|SetVisibility (Variables|Default|Getplaca1) false false)
    (Rendering|SetVisibility (Variables|Default|Getplaca2) false false)
    (Rendering|SetVisibility (Variables|Default|Getdisplay) false false)
    (CallFunction|SlotRespostasErradas)
    (else
      (Development|PrintString "errou")
      (Variables|Default|Setvida (- (Variables|Default|Getvida) 3))
      (if (<= (Variables|Default|Getvida) 0)
        (Variables|Default|Setvida 0)
        (CallFunction|EndGame)))))

(event EventBeginPlay
  (bind _asplayer_controller (Utilities|Casting|CastToPlayerController (Pawn|GetController)))
  (Utilities|IsValid (PlayerController|LocalPlayerSubsystems|GetEnhancedInputLocalPlayerSubsystem _asplayer_controller)
    (:Is%20Valid
      (Input|AddMappingContext (PlayerController|LocalPlayerSubsystems|GetEnhancedInputLocalPlayerSubsystem _asplayer_controller) "/Game/Input/IMC_default.IMC_default" 0 "(bIgnoreAllPressedKeysUntilRelease=True,bForceImmediately=False,bNotifyUserSettings=False)")
      (CallFunction|SlotRespostasErradas))))

(event Collision|EventActorBeginOverlap
  (params (OtherActor :type Actor%20Object%20Reference)))

(event EventTick
  (params (DeltaSeconds :type Float%20%28single-precision%29))
  (Variables|Default|SetDelta%20Seconds DeltaSeconds))

(fn ConstructionScript)

(fn SlotRespostasErradas
  ;[1 1 1] Determinando Resposta Correta
  (Variables|Default|SetNumero (Math|Random|RandomIntegerinRange 0 9))
  ;[1 1 1] determinando entre as variáveis, se a resposta correta será a maior, do meio ou menor
  (Variables|Default|SetShiftRespostas (Math|Random|RandomInteger 3))
  (if (== (Variables|Default|GetShiftRespostas) 0)
    (Variables|Default|SetRespostaErrada_1 (+ (Variables|Default|GetNumero) 1))
    (Variables|Default|SetRespostaErrada_2 (+ (Variables|Default|GetNumero) 2))
    ;[1 1 1] corrigindo respostaErrada_1 fora do Intervalo de 0 a 9
    (if (> (Variables|Default|GetRespostaErrada_1) 9) :!label _label
      (Variables|Default|SetRespostaErrada_1 (- (Variables|Default|GetRespostaErrada_1) 10))
      (elif (< (Variables|Default|GetRespostaErrada_1) 0)
        (Variables|Default|SetRespostaErrada_1 (+ (Variables|Default|GetRespostaErrada_1) 10))))
    ;[1 1 1] corrigindo respostaErrada_2 fora do Intervalo de 0 a 9
    (if (> (Variables|Default|GetRespostaErrada_2) 9)
      (Variables|Default|SetRespostaErrada_2 (- (Variables|Default|GetRespostaErrada_2) 10))
      (elif (< (Variables|Default|GetRespostaErrada_2) 0)
        (Variables|Default|SetRespostaErrada_2 (+ (Variables|Default|GetRespostaErrada_2) 10))))
    ;[1 1 1] Escolhendo o Slot
    (Variables|Default|SetRespostaSlot (Math|Random|RandomInteger 3))
    (bind _output_get (Variables|Default|SetSlot (Math|Random|RandomIntegerinRange 0 2)))
    (if (== (Variables|Default|GetSlot) 0)
      (Rendering|Material|SetScalarParameterValue "/Game/MaterialContas/MPC_respostas.MPC_respostas" "RespShift_0" (Math|Conversions|ToFloat(Integer) (Variables|Default|GetNumero)) :!class /Script/Engine.KismetMaterialLibrary)
      (Rendering|Material|SetScalarParameterValue "/Game/MaterialContas/MPC_respostas.MPC_respostas" "RespShift_1" (Math|Conversions|ToFloat(Integer) (Variables|Default|GetRespostaErrada_1)) :!class /Script/Engine.KismetMaterialLibrary)
      (Rendering|Material|SetScalarParameterValue "/Game/MaterialContas/MPC_respostas.MPC_respostas" "RespShift_2" (Math|Conversions|ToFloat(Integer) (Variables|Default|GetRespostaErrada_2)) :!class /Script/Engine.KismetMaterialLibrary)
      (for (_ _array_index) (Variables|Default|GetNumString) :!label _label_2
        (if (== (Variables|Default|GetNumero) _array_index)
          (Rendering|Material|SetScalarParameterValue "/Game/MaterialContas/MPC_equacoes.MPC_equacoes" (Utilities|Array|Get(acopy) (Variables|Default|GetRespString) _array_index) 1.0 :!class /Script/Engine.KismetMaterialLibrary)
          (else
            (Rendering|Material|SetScalarParameterValue "/Game/MaterialContas/MPC_equacoes.MPC_equacoes" (Utilities|Array|Get(acopy) (Variables|Default|GetRespString) _array_index) 0.0 :!class /Script/Engine.KismetMaterialLibrary)))
        (Rendering|Material|SetScalarParameterValue "/Game/MaterialContas/MPC_equacoes.MPC_equacoes" "Utile" (/ (Math|Conversions|ToFloat(Integer) (Math|Random|RandomInteger 6)) 5.0) :!class /Script/Engine.KismetMaterialLibrary)
        (Rendering|Material|SetScalarParameterValue "/Game/MaterialContas/MPC_equacoes.MPC_equacoes" "Vtile" (/ (Math|Conversions|ToFloat(Integer) (Math|Random|RandomInteger 6)) 5.0) :!class /Script/Engine.KismetMaterialLibrary))
      (elif (== (Variables|Default|GetSlot) 1)
        (Rendering|Material|SetScalarParameterValue "/Game/MaterialContas/MPC_respostas.MPC_respostas" "RespShift_0" (Math|Conversions|ToFloat(Integer) (Variables|Default|GetRespostaErrada_2)) :!class /Script/Engine.KismetMaterialLibrary)
        (Rendering|Material|SetScalarParameterValue "/Game/MaterialContas/MPC_respostas.MPC_respostas" "RespShift_1" (Math|Conversions|ToFloat(Integer) (Variables|Default|GetNumero)) :!class /Script/Engine.KismetMaterialLibrary)
        (Rendering|Material|SetScalarParameterValue "/Game/MaterialContas/MPC_respostas.MPC_respostas" "RespShift_2" (Math|Conversions|ToFloat(Integer) (Variables|Default|GetRespostaErrada_1)) :!class /Script/Engine.KismetMaterialLibrary)
        (goto _label_2)
        (elif (== (Variables|Default|GetSlot) 2)
          (Rendering|Material|SetScalarParameterValue "/Game/MaterialContas/MPC_respostas.MPC_respostas" "RespShift_0" (Math|Conversions|ToFloat(Integer) (Variables|Default|GetRespostaErrada_1)) :!class /Script/Engine.KismetMaterialLibrary)
          (Rendering|Material|SetScalarParameterValue "/Game/MaterialContas/MPC_respostas.MPC_respostas" "RespShift_1" (Math|Conversions|ToFloat(Integer) (Variables|Default|GetRespostaErrada_2)) :!class /Script/Engine.KismetMaterialLibrary)
          (Rendering|Material|SetScalarParameterValue "/Game/MaterialContas/MPC_respostas.MPC_respostas" "RespShift_2" (Math|Conversions|ToFloat(Integer) (Variables|Default|GetNumero)) :!class /Script/Engine.KismetMaterialLibrary)
          (goto _label_2))))
    (elif (== (Variables|Default|GetShiftRespostas) 1)
      (Variables|Default|SetRespostaErrada_1 (- (Variables|Default|GetNumero) 1))
      (Variables|Default|SetRespostaErrada_2 (+ (Variables|Default|GetNumero) 1))
      (goto _label)
      (elif (== (Variables|Default|GetShiftRespostas) 2)
        (Variables|Default|SetRespostaErrada_1 (- (Variables|Default|GetNumero) 2))
        (Variables|Default|SetRespostaErrada_2 (- (Variables|Default|GetNumero) 1))
        (goto _label)))))

(fn SlotesRespostasErradas)

(fn EndGame)