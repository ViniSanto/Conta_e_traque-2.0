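; First-person player Blueprint that handles mouse-look and movement through Enhanced Input, adding the default mapping context on BeginPlay.
; Look yaws the capsule and pitches the camera within limits; move input follows capsule axes and toggles the Andando (walking) flag.
; SlotRespostasErradas is empty: its disconnected, never-run graph picks a random correct digit, two neighbouring wrong answers and an answer slot, then writes them to material scalar parameters.
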(event Input|EnhancedActionEvents|EnhancedInputActionIA_move
  (params (ActionValue :type Vector%202D%20Structure) (ElapsedSeconds :type Float%20%28double-precision%29) (TriggeredSeconds :type Float%20%28double-precision%29) (InputAction :type Input%20Action%20Object%20Reference :default "/Game/Input/Action/IA_move.IA_move"))
  (:Triggered
    (Pawn|Input|AddMovementInput (Math|Vector|GetRightVector (Variables|Collision|GetCapsuleComponent)) (.x ActionValue) false)
    (Pawn|Input|AddMovementInput (Math|Vector|GetForwardVector (Variables|Collision|GetCapsuleComponent)) (.y ActionValue) false))
  (:Started
    (Variables|Default|SetAndando true))
  (:Completed
    (Variables|Default|SetAndando false)))

(event Input|EnhancedActionEvents|EnhancedInputActionIA_look
  (params (ActionValue :type Vector%202D%20Structure) (ElapsedSeconds :type Float%20%28double-precision%29) (TriggeredSeconds :type Float%20%28double-precision%29) (InputAction :type Input%20Action%20Object%20Reference :default "/Game/Input/Action/IA_look.IA_look"))
  (bind _returnvalue (* (.y ActionValue) -1.0))
  (Transformation|AddLocalRotation (Variables|Collision|GetCapsuleComponent) (Math|Rotator|MakeRotator 0.0 0.0 (.x ActionValue)) false false)
  (if (> _returnvalue 0.0)
    (if (< (.pitch (Transformation|GetWorldRotation (Variables|Default|GetCamera))) 85.0)
      (Transformation|AddLocalRotation (Variables|Default|GetCamera) (Math|Rotator|MakeRotator 0.0 _returnvalue 0.0) false false))
    (elif (> (.pitch (Transformation|GetWorldRotation (Variables|Default|GetCamera))) -85.0)
      (Transformation|AddLocalRotation (Variables|Default|GetCamera) (Math|Rotator|MakeRotator 0.0 _returnvalue 0.0) false false))))

(event EventBeginPlay
  (bind _asplayer_controller (Utilities|Casting|CastToPlayerController (Pawn|GetController)))
  (Utilities|IsValid (PlayerController|LocalPlayerSubsystems|GetEnhancedInputLocalPlayerSubsystem _asplayer_controller)
    (:Is%20Valid
      (Input|AddMappingContext (PlayerController|LocalPlayerSubsystems|GetEnhancedInputLocalPlayerSubsystem _asplayer_controller) "/Game/Input/IMC_default.IMC_default" 0 "(bIgnoreAllPressedKeysUntilRelease=True,bForceImmediately=False,bNotifyUserSettings=False)"))))

(event Collision|EventActorBeginOverlap
  (params (OtherActor :type Actor%20Object%20Reference)))

(event EventTick
  (params (DeltaSeconds :type Float%20%28single-precision%29)))

(fn ConstructionScript)

(fn SlotRespostasErradas)